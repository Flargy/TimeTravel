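; BP_TimeBall_2 is a Blueprint that saves and rewinds custom data, a vector that grows over time on Tick, through events from its Time component.
; Save events append the vector to an array, and load events interpolate between adjacent recorded frames.
; Ending a rewind snaps to the given frame, with debug prints at rewind begin and end.
; Cleanup trims the oldest entries from the array's front.
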(event SaveData(Time)
  (CallFunction|SaveCustomData))

(event LoadData(Time)
  (params (FrameIndex :type Integer) (LerpValue :type Float%20%28single-precision%29))
  (CallFunction|LoadCustomData FrameIndex LerpValue))

(event EndRewind(Time)
  (params (FrameIndex :type Integer))
  (CallFunction|EndCustomRewind FrameIndex))

(event BeginRewind(Time)
  (CallFunction|BeginCustomRewind))

(event CleanupArray(Time)
  (params (FrameIndex :type Integer))
  (Utilities|GenericArray (Variables|Default|GetCustomDataArray) FrameIndex))

(event EventBeginPlay)

(event Collision|EventActorBeginOverlap
  (params (OtherActor :type Actor%20Object%20Reference)))

(event EventTick
  (params (DeltaSeconds :type Float%20%28single-precision%29))
  (Variables|Default|SetCustomVector (+ (Variables|Default|GetCustomVector) (* (Class|KismetMathLibrary|VectorOne) DeltaSeconds))))

(fn ConstructionScript)

(fn SaveCustomData
  (Utilities|Array|Add (Variables|Default|GetCustomDataArray) (Variables|Default|GetCustomVector)))

(fn LoadCustomData
  (params (FrameIndex :type Integer) (LerpT :type Float%20%28single-precision%29))
  (bind _customdataarray (Variables|Default|GetCustomDataArray))
  (Variables|Default|SetCustomVector (Math|Vector|Lerp(Vector) (Utilities|Array|Get(acopy) _customdataarray FrameIndex) (Utilities|Array|Get(acopy) _customdataarray (+ FrameIndex 1)) LerpT)))

(fn EndCustomRewind
  (params (CurrentFrame :type Integer))
  (bind _output_get (Variables|Default|SetCustomVector (Utilities|Array|Get(acopy) (Variables|Default|GetCustomDataArray) CurrentFrame)))
  (Development|PrintString (Utilities|String|ToString(Vector) _output_get) true true "(R=0.932055,G=0.124008,B=1.000000,A=1.000000)" 0.0))

(fn BeginCustomRewind
  (Development|PrintString (Utilities|String|ToString(Vector) (Variables|Default|GetCustomVector)) true true "(R=0.000000,G=0.660000,B=1.000000,A=1.000000)" 0.0))